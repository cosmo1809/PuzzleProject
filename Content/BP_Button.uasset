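; BP_Button is a floor-style toggle button that switches on or off each time something steps into its PressDetection volume.
; A SteppedOn flag limits toggling to one per step until an overlap ends.
; Each press flips IsOn, updates the Pressed scalar on a dynamic M_Button material created at BeginPlay, and plays a higher- or lower-pitched click.
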(event OnComponentBeginOverlap(PressDetection)
  (params (OverlappedComponent :type Primitive%20Component%20Object%20Reference) (OtherActor :type Actor%20Object%20Reference) (OtherComp :type Primitive%20Component%20Object%20Reference) (OtherBodyIndex :type Integer) (bFromSweep :type Boolean) (SweepResult :type Hit%20Result%20Structure%20%28by%20ref%29))
  (if (not (Variables|Default|GetSteppedOn))
    (Variables|Default|SetSteppedOn true)
    (CallFunction|PressButton)))

(event OnComponentEndOverlap(PressDetection)
  (params (OverlappedComponent :type Primitive%20Component%20Object%20Reference) (OtherActor :type Actor%20Object%20Reference) (OtherComp :type Primitive%20Component%20Object%20Reference) (OtherBodyIndex :type Integer))
  (Variables|Default|SetSteppedOn false))

(event Custom|PressButton
  (bind _returnvalue (Transformation|GetActorLocation))
  (bind _output_get (Variables|Default|SetIsOn (not (Variables|Default|GetIsOn))))
  (Rendering|Material|SetScalarParameterValue (Variables|Default|GetButtonColour) "Pressed" (Math|Conversions|ToFloat(Boolean) _output_get) :!class /Script/Engine.MaterialInstanceDynamic)
  (if (Variables|Default|GetIsOn)
    (Audio|PlaySoundatLocation "/Game/SciFiUISFX/Wavs/Clicks/Click_Pitched_Up_Wav.Click_Pitched_Up_Wav" _returnvalue "0, 0, 0" 1.0 1.0 0.0 0 0 0 0)
    (else
      (Audio|PlaySoundatLocation "/Game/SciFiUISFX/Wavs/Clicks/Click_Pitched_Down_Wav.Click_Pitched_Down_Wav" _returnvalue "0, 0, 0" 1.0 1.0 0.0 0 0 0 0))))

(event EventBeginPlay
  (bind _returnvalue (Rendering|Material|CreateDynamicMaterialInstance (Variables|Default|GetButton) 0 "/Game/M_Button.M_Button" "None" :!class /Script/Engine.PrimitiveComponent))
  (bind _output_get (Variables|Default|SetButtonColour _returnvalue))
  (Rendering|Material|SetScalarParameterValue _output_get "Pressed" (Math|Conversions|ToFloat(Boolean) (Variables|Default|GetIsOn)) :!class /Script/Engine.MaterialInstanceDynamic))

(fn ConstructionScript)
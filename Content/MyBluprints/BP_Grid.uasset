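; Grid manager for a Lights Out style puzzle, where pressing a button toggles it and its four orthogonal neighbours.
; BeginPlay spawns the buttons row by row into a flat array, giving each its coordinates and a reference to the grid.
; HandlePress passes a button's coordinates to PressAt, which toggles through bounds-checked lookups using X + Y * width indexing.
; Each press then checks for all buttons on and prints a win message.
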(event Custom|ToggleAt
  (params (X :type Integer) (Y :type Integer))
  (bind _button (CallFunction|GetButton X Y))
  (if (!= _button 0)
    (Default|PressButton _button)))

(event Custom|PressAt
  (params (X :type Integer) (Y :type Integer))
  (CallFunction|Toggleat X Y)
  (CallFunction|Toggleat (- X 1) Y)
  (CallFunction|Toggleat (+ X 1) Y)
  (CallFunction|Toggleat X (- Y 1))
  (CallFunction|Toggleat X (+ Y 1))
  (CallFunction|CheckforWin))

(event Custom|HandlePress
  (params (Button :type BP%20Button%20Object%20Reference))
  (CallFunction|Pressat (Variables|/Game/MyBluprints/BP_Button.BP_Button_C|GetGridX Button) (Variables|/Game/MyBluprints/BP_Button.BP_Button_C|GetGridY Button)))

(event Custom|CheckForWin
  (Variables|Default|SetAllOn true)
  (bind _array_element (Utilities|Array|ForEachLoopwithBreak (Variables|Default|GetButtons) :!label _label)
    (:LoopBody
      (if (not (Variables|/Game/MyBluprints/BP_Button.BP_Button_C|GetIsOn _array_element))
        (Variables|Default|SetAllOn false)
        (goto _label Break)))
    (:Completed
      (if (Variables|Default|GetAllOn)
        (Development|PrintString "Well Done !!")))))

(event EventBeginPlay
  (Utilities|Array|Clear (Variables|Default|GetButtons))
  (for _index (range 0 (- (Variables|Default|GetGridHeight) 1))
    (Variables|Default|SetLoopY _index)
    (for _index_2 (range 0 (- (Variables|Default|GetGridWidth) 1))
      (Variables|Default|SetLoopX _index_2)
      (bind _index_3 (CallFunction|GetIndex _index_2 _index))
      (bind _returnvalue (Game|SpawnActorfromClass (Variables|Default|GetButtonClassReference) (Math|Transform|MakeTransform (Math|Vector|MakeVector (+ (* (Variables|Default|GetLoopX) (+ (Variables|Default|GetSpacing) (Variables|Default|GetButtonSize))) (.x (Transformation|GetActorLocation (Utilities|Array|Get(acopy) (Variables|Default|GetButtons) _index_3)))) (+ (* (Variables|Default|GetLoopY) (+ (Variables|Default|GetSpacing) (Variables|Default|GetButtonSize))) (.y (Transformation|GetActorLocation (Utilities|Array|Get(acopy) (Variables|Default|GetButtons) _index_3)))) 0.0)) "AlwaysSpawn" "MultiplyWithRoot" 0 0 0))
      (Variables|/Game/MyBluprints/BP_Button.BP_Button_C|SetGridX _returnvalue (Variables|Default|GetLoopX))
      (Variables|/Game/MyBluprints/BP_Button.BP_Button_C|SetGridY _returnvalue (Variables|Default|GetLoopY))
      (Variables|/Game/MyBluprints/BP_Button.BP_Button_C|SetGrid _returnvalue self)
      (Utilities|Array|Add (Variables|Default|GetButtons) _returnvalue))))

(fn ConstructionScript)

(fn GetIndex
  (params (X :type Integer) (Y :type Integer))
  (return (+ X (* Y (Variables|Default|GetGridWidth)))))

(fn IsValidCoordinate
  (params (X :type Integer) (Y :type Integer))
  (return (and (and (>= X 0) (< X (Variables|Default|GetGridWidth))) (and (>= Y 0) (< Y (Variables|Default|GetGridHeight))))))

(fn GetButton
  (params (X :type Integer) (Y :type Integer))
  (bind _valid (CallFunction|IsValidCoordinate X Y))
  (if _valid
    (bind _index (CallFunction|GetIndex X Y))
    (return (Utilities|Array|Get(acopy) (Variables|Default|GetButtons) _index))
    (else
      (return 0))))
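; BP_Shield is a shield actor with a sphere that can be switched off through its DisableShield event.
; BeginPlay caches the start location and an end point below it.
; DisableShield plays a sound, removes sphere collision and turns the shield green through a dynamic material instance.
; A timeline then lerps the actor down to the end point and hides it when finished.
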(event Custom|Disable%20Shield
  ;[0.15 0.15 0.15 0.5] When shield is disabled a sound effect is played, collision is turned off, a material instance is created and its colour is set to green
  (Audio|PlaySoundatLocation "/Engine/EditorSounds/GamePreview/EndSimulate.EndSimulate" (Transformation|GetActorLocation) "0, 0, 0" 1.0 1.0 0.0 0 0 0 0)
  (Collision|SetCollisionEnabled (Variables|Default|GetSphere) "NoCollision")
  (bind _returnvalue (Rendering|Material|CreateDynamicMaterialInstance (Variables|Default|GetSphere) 0 "/Game/MyMaterials/M_Shield2.M_Shield2" "None" :!class /Script/Engine.PrimitiveComponent))
  (bind _output_get (Variables|Default|SetShieldColourReference _returnvalue))
  (Rendering|Material|SetVectorParameterValue _output_get "ShieldColour" (Math|Color|MakeColor 0.0 1.0 0.0) :!class /Script/Engine.MaterialInstanceDynamic)
  (bind _alpha (Timeline|TL_RetractShield PlayFromStart)
    (:Update
      (Transformation|SetActorLocation (Math|Vector|Lerp(Vector) (Variables|Default|GetStartLocation) (Variables|Default|GetEndLocation) _alpha) false true))
    (:Finished
      (Rendering|SetActorHiddenInGame true))))

(event EventBeginPlay
  (bind _output_get (Variables|Default|SetStartLocation (Transformation|GetActorLocation)))
  (Variables|Default|SetEndLocation (- _output_get (Math|Vector|MakeVector 0.0 0.0 2.5e+02))))

(fn ConstructionScript)